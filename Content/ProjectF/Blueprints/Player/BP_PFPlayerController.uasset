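; BP_PFPlayerController is the player controller that toggles the pause menu from the IA_Pause input action.
; Pausing creates a new WBP_PauseMenu, adds it to the viewport, switches to game-and-UI input, shows the cursor and pauses the game.
; Unpausing removes and hides the stored widget and restores game-only input without a cursor.
; BeginPlay is empty, and the node adding IMC_Default is unconnected, so it never runs.
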(event `EnhancedInput|/Game/ProjectF/Input/Actions/IA_Pause`
  (params (ActionValue :type Boolean) (ElapsedSeconds :type "Float (double-precision)") (TriggeredSeconds :type "Float (double-precision)") (InputAction :type "InputAction Object Reference" :default "/Game/ProjectF/Input/Actions/IA_Pause.IA_Pause"))
  (:`Started`
    (if (`GameplayStatics.IsGamePaused`)
      (`Widget.RemoveFromParent` (`self.PauseMenuWidget`))
      (`GameplayStatics.SetGamePaused` false)
      (`Widget.SetVisibility` (`self.PauseMenuWidget`) "Hidden")
      (`WidgetBlueprintLibrary.SetInputMode_GameOnly` self)
      (set `self.bShowMouseCursor` false)
      (else
        (bind _returnvalue (`|CreateWidget` "/Game/ProjectF/Blueprints/UI/WBP_PauseMenu.WBP_PauseMenu_C" self))
        (bind _output_get (set `self.PauseMenuWidget` _returnvalue))
        (`UserWidget.AddToViewport` _output_get 1)
        (`WidgetBlueprintLibrary.SetInputMode_GameAndUIEx` self (`self.PauseMenuWidget`))
        (set `self.bShowMouseCursor` true)
        (`GameplayStatics.SetGamePaused` true)))))

(event `self.ReceiveBeginPlay`)

(fn `UserConstructionScript`)